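; BP_Card is an interactable card pickup that highlights and shows a text prompt while the first-person character overlaps its box.
; Overlap toggles custom depth on the mesh and text visibility, and starts a looping, self-referencing timer that turns the text toward the player, with no clear on exit.
; ObjectInteraction finds BP_Datapad and, if valid, calls PickupCard on it and the character, then destroys the card.
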(event `self.Box.OnComponentBeginOverlap`
  (params (OverlappedComponent :type "PrimitiveComponent Object Reference") (OtherActor :type "Actor Object Reference") (OtherComp :type "PrimitiveComponent Object Reference") (OtherBodyIndex :type Integer) (bFromSweep :type Boolean) (SweepResult :type "HitResult Structure (by ref)"))
  (cast `/Game/FirstPerson/Blueprints/BP_FirstPersonCharacter` OtherActor)
  (`PrimitiveComponent.SetRenderCustomDepth` (`self.StaticMesh`) true)
  (`SceneComponent.SetVisibility` (`self.Text Render`) true false)
  (`self.Show E Interact`))

(event `self.Box.OnComponentEndOverlap`
  (params (OverlappedComponent :type "PrimitiveComponent Object Reference") (OtherActor :type "Actor Object Reference") (OtherComp :type "PrimitiveComponent Object Reference") (OtherBodyIndex :type Integer))
  (cast `/Game/FirstPerson/Blueprints/BP_FirstPersonCharacter` OtherActor)
  (`PrimitiveComponent.SetRenderCustomDepth` (`self.StaticMesh`) false)
  (`SceneComponent.SetVisibility` (`self.Text Render`) false false))

(event `/Game/Blueprints/BP_Object_Interactions_Interface.Object_Interaction`
  ;[1 1 1] Pickup Card Interactions
  (bind _returnvalue (`GameplayStatics.GetActorOfClass` "/Game/Blueprints/BP_Datapad.BP_Datapad_C"))
  (`/Engine/EditorBlueprintResources/StandardMacros.IsValid` _returnvalue
    (:`Is Valid`
      (`/Game/Blueprints/BP_Object_Interactions_Interface.Pickup_Card` _returnvalue)
      (bind _returnvalue_2 (`GameplayStatics.GetActorOfClass` "/Game/FirstPerson/Blueprints/BP_FirstPersonCharacter.BP_FirstPersonCharacter_C"))
      (`/Game/Blueprints/BP_Object_Interactions_Interface.Pickup_Card` _returnvalue_2)
      (`self.K2_DestroyActor`))))

(event `Show E Interact`
  (bind _text_render (`self.Text Render`))
  ;[1 1 1] Text Facing Player
  (`KismetSystemLibrary.K2_SetTimerDelegate` (delegate `Show E Interact`) 0.03 true)
  (`SceneComponent.K2_SetRelativeRotation` _text_render (`KismetMathLibrary.FindLookAtRotation` (`SceneComponent.K2_GetComponentLocation` _text_render) (`self.K2_GetActorLocation` (`GameplayStatics.GetPlayerPawn` 0))) false false))

(fn `UserConstructionScript`)