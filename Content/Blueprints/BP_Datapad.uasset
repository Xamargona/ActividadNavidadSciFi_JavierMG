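; Datapad interactable that, once powered and with a card picked up, lets the player insert an access card.
; Box overlap shows the prompt text and custom-depth highlight when both flags are set.
; A looping timer re-runs ShowEInteract to turn the text toward the player.
; Interaction runs once, removing the player's card, triggering a camera move, then after a delay sliding the card mesh along X by Timeline before hiding it.
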(event `self.ReceiveBeginPlay`
  (`SceneComponent.SetHiddenInGame` (`self.SM_AccessCard`) true false))

(event `/Game/Blueprints/BP_Object_Interactions_Interface.Datapad_Activation`
  (set `self.Has Energy` true))

(event `/Game/Blueprints/BP_Object_Interactions_Interface.Pickup_Card`
  (set `self.Has Card` true))

(event `self.Box.OnComponentBeginOverlap`
  (params (OverlappedComponent :type "PrimitiveComponent Object Reference") (OtherActor :type "Actor Object Reference") (OtherComp :type "PrimitiveComponent Object Reference") (OtherBodyIndex :type Integer) (bFromSweep :type Boolean) (SweepResult :type "HitResult Structure (by ref)"))
  ;[1 1 1] Show Overlay Only With Energy && Card // Hide overlay
  (bind _asbp_first_person_character (cast `/Game/FirstPerson/Blueprints/BP_FirstPersonCharacter` OtherActor))
  (set `self.As BP First Person Character` _asbp_first_person_character)
  (if (`self.Has Energy`)
    (if (`self.Has Card`)
      (if (not (`self.Dont Show Text`))
        (`SceneComponent.SetVisibility` (`self.Text Render`) true false)
        (`self.Show E Interact`)
        (`PrimitiveComponent.SetRenderCustomDepth` (`self.SM_Datapad`) true)))))

(event `self.Box.OnComponentEndOverlap`
  (params (OverlappedComponent :type "PrimitiveComponent Object Reference") (OtherActor :type "Actor Object Reference") (OtherComp :type "PrimitiveComponent Object Reference") (OtherBodyIndex :type Integer))
  ;[1 1 1] Show Overlay Only With Energy && Card // Hide overlay
  (cast `/Game/FirstPerson/Blueprints/BP_FirstPersonCharacter` OtherActor)
  (`SceneComponent.SetVisibility` (`self.Text Render`) false false)
  (`PrimitiveComponent.SetRenderCustomDepth` (`self.SM_Datapad`) false))

(event `Show E Interact`
  (bind _text_render (`self.Text Render`))
  ;[1 1 1] Text Facing Player
  (`KismetSystemLibrary.K2_SetTimerDelegate` (delegate `Show E Interact`) 0.03 true)
  (`SceneComponent.K2_SetRelativeRotation` _text_render (`KismetMathLibrary.FindLookAtRotation` (`SceneComponent.K2_GetComponentLocation` _text_render) (`self.K2_GetActorLocation` (`GameplayStatics.GetPlayerPawn` 0))) false false))

(event `/Game/Blueprints/BP_Object_Interactions_Interface.Object_Interaction`
  (bind _sm_accesscard (`self.SM_AccessCard`))
  (bind _returnvalue (`SceneComponent.GetRelativeTransform` _sm_accesscard))
  ;[1 1 1] Interact
  (if (`self.Has Card`)
    (if (`self.Has Energy`)
      (`/Engine/EditorBlueprintResources/StandardMacros.DoOnce` false
        (:`Completed`
          (`SceneComponent.SetVisibility` (`self.Text Render`) false false)
          (set `self.Dont Show Text` true)
          (`/Game/Blueprints/BP_Object_Interactions_Interface.Remove_Card` (`self.As BP First Person Character`))
          (`PrimitiveComponent.SetRenderCustomDepth` (`self.SM_Datapad`) false)
          (`/Game/Blueprints/BP_Object_Interactions_Interface.Move_Camera` (`self.As BP First Person Character`))
          (`KismetSystemLibrary.Delay` 3.0)
          (`SceneComponent.SetHiddenInGame` (`self.SM_AccessCard`) false false)
          (bind (_direction _movement) (`Timeline|Timeline` :!via `PlayFromStart`)
            (:`Update`
              (`SceneComponent.K2_SetRelativeLocation` _sm_accesscard (`KismetMathLibrary.MakeVector` _movement (.y (.location _returnvalue)) (.z (.location _returnvalue))) false false))
            (:`Finished`
              (`SceneComponent.SetHiddenInGame` (`self.SM_AccessCard`) true false))))))))

(fn `UserConstructionScript`)