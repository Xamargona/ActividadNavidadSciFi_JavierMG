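; BP_Terminal is an interactable terminal that, once powered, plays a screen sequence that activates every BP_Datapad in the level.
; TerminalActivation grants energy and turns the screen white, enabling an overlap-driven prompt with a custom-depth highlight and timer-based rotation toward the player.
; ObjectInteraction suppresses the prompt, then drives the screen material's Color through two timelines, the second starting after a delay and triggering the datapads once.
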(event `self.ReceiveBeginPlay`
  (`MeshComponent.SetVectorParameterValueOnMaterials` (`self.Screen`) "Color" (0.0 0.0 0.0)) ; Initial Screen Setup
)

(event `/Game/Blueprints/BP_Object_Interactions_Interface.Terminal_Activation`
  ;[1 1 1] Activate Screen && Terminal
  (set `self.Has Energy` true)
  (`MeshComponent.SetVectorParameterValueOnMaterials` (`self.Screen`) "Color" (1.0 1.0 1.0)))

(event `self.Box.OnComponentBeginOverlap`
  (params (OverlappedComponent :type "PrimitiveComponent Object Reference") (OtherActor :type "Actor Object Reference") (OtherComp :type "PrimitiveComponent Object Reference") (OtherBodyIndex :type Integer) (bFromSweep :type Boolean) (SweepResult :type "HitResult Structure (by ref)"))
  ;[1 1 1] Show Overlay Only With Energy // Hide overlay
  (cast `/Game/FirstPerson/Blueprints/BP_FirstPersonCharacter` OtherActor)
  (if (`self.Has Energy`)
    (if (not (`self.DontShowText`))
      (`SceneComponent.SetVisibility` (`self.Text Render`) true false)
      (`self.Show E Interact`)
      (`PrimitiveComponent.SetRenderCustomDepth` (`self.Terminal`) true))))

(event `self.Box.OnComponentEndOverlap`
  (params (OverlappedComponent :type "PrimitiveComponent Object Reference") (OtherActor :type "Actor Object Reference") (OtherComp :type "PrimitiveComponent Object Reference") (OtherBodyIndex :type Integer))
  ;[1 1 1] Show Overlay Only With Energy // Hide overlay
  (cast `/Game/FirstPerson/Blueprints/BP_FirstPersonCharacter` OtherActor)
  (`SceneComponent.SetVisibility` (`self.Text Render`) false false)
  (`PrimitiveComponent.SetRenderCustomDepth` (`self.Terminal`) false))

(event `Show E Interact`
  (bind _text_render (`self.Text Render`))
  ;[1 1 1] Text Facing Player
  (`KismetSystemLibrary.K2_SetTimerDelegate` (delegate `Show E Interact`) 0.03 true)
  (`SceneComponent.K2_SetRelativeRotation` _text_render (`KismetMathLibrary.FindLookAtRotation` (`SceneComponent.K2_GetComponentLocation` _text_render) (`self.K2_GetActorLocation` (`GameplayStatics.GetPlayerPawn` 0))) false false))

(event `/Game/Blueprints/BP_Object_Interactions_Interface.Object_Interaction`
  (bind _screen (`self.Screen`))
  ;[1 1 1] Interaction
  (if (`self.Has Energy`)
    (`SceneComponent.SetVisibility` (`self.Text Render`) false false)
    (set `self.DontShowText` true)
    (`PrimitiveComponent.SetRenderCustomDepth` (`self.Terminal`) false)
    (bind (_direction _opacity_values) (`Timeline|Timeline` :!via `PlayFromStart`)
      (:`Update`
        (`MeshComponent.SetVectorParameterValueOnMaterials` _screen "Color" (`KismetMathLibrary.MakeVector` _opacity_values _opacity_values _opacity_values)))
      (:`Finished`
        (`KismetSystemLibrary.Delay` 1.0)
        (bind (_direction_2 _red) (`Timeline|Timeline_0` :!via `PlayFromStart`)
          (:`Update`
            (`MeshComponent.SetVectorParameterValueOnMaterials` _screen "Color" _red)
            (`/Engine/EditorBlueprintResources/StandardMacros.DoOnce` false
              (:`Completed`
                (bind _outactors (`GameplayStatics.GetAllActorsOfClass` "/Game/Blueprints/BP_Datapad.BP_Datapad_C"))
                (for _array_element _outactors
                  (`/Game/Blueprints/BP_Object_Interactions_Interface.Datapad_Activation` _array_element))))))))))

(fn `UserConstructionScript`)