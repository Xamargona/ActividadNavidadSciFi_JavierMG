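; Battery socket that accepts a grippable active battery and powers up the level's terminals.
; When a static mesh component enters its Box trigger and belongs to a BP_Grippable_Active_Battery, that battery actor is destroyed.
; The socket's own mesh then switches to energy core, emissive and pipe materials to stand in for the battery.
; It finally calls TerminalActivation on every BP_Terminal in the world.
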(event `self.Box.OnComponentBeginOverlap`
  (params (OverlappedComponent :type "PrimitiveComponent Object Reference") (OtherActor :type "Actor Object Reference") (OtherComp :type "PrimitiveComponent Object Reference") (OtherBodyIndex :type Integer) (bFromSweep :type Boolean) (SweepResult :type "HitResult Structure (by ref)"))
  (bind _staticmesh (`self.StaticMesh`))
  (bind _asstatic_mesh_component (cast `StaticMeshComponent` OtherComp))
  (bind _output_get (set `self.Overlapped component` _asstatic_mesh_component))
  (set `self.New Static Mesh` _asstatic_mesh_component)
  (bind _asbp_grippable_active_battery (cast `/Game/Blueprints/BP_Grippable_Active_Battery` (`ActorComponent.GetOwner` _output_get)))
  (`self.K2_DestroyActor` _asbp_grippable_active_battery)
  (`PrimitiveComponent.SetMaterial` _staticmesh 0 "/Game/StarterBundle/ModularScifiHallways/Materials/MI_EnergyCore_A_M.MI_EnergyCore_A_M")
  (`PrimitiveComponent.SetMaterial` _staticmesh 1 "/Game/StarterBundle/ModularScifiHallways/Materials/MI_EnergyEmissive_A.MI_EnergyEmissive_A")
  (`PrimitiveComponent.SetMaterial` _staticmesh 2 "/Game/StarterBundle/ModularScifiHallways/Materials/MI_Pipes_ADark_M.MI_Pipes_ADark_M")
  (bind _outactors (`GameplayStatics.GetAllActorsOfClass` "/Game/Blueprints/BP_Terminal.BP_Terminal_C"))
  (for _array_element _outactors
    (`/Game/Blueprints/BP_Object_Interactions_Interface.Terminal_Activation` _array_element)))

(fn `UserConstructionScript`)