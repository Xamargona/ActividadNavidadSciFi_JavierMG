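; Battery prop that shows an interaction prompt and custom-depth highlight while the first-person character is inside its box trigger.
; BeginPlay attaches the box and text to the static mesh so they move with it.
; A looping timer keeps turning the prompt toward the player once it has been shown.
; ObjectInteraction hides the text and toggles a suppression flag, showing the prompt again when suppression clears.
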(event `self.ReceiveBeginPlay`
  (`SceneComponent.K2_AttachToComponent` (`self.Box`) (`self.StaticMesh`) "None" "KeepRelative" "KeepRelative" "KeepRelative" true) ; Attach components for movement
  (`SceneComponent.K2_AttachToComponent` (`self.Text Render`) (`self.StaticMesh`) "None" "KeepRelative" "KeepRelative" "KeepRelative" true)
  (`PrimitiveComponent.SetRenderCustomDepth` (`self.StaticMesh`) false))

(event `self.Box.OnComponentBeginOverlap`
  (params (OverlappedComponent :type "PrimitiveComponent Object Reference") (OtherActor :type "Actor Object Reference") (OtherComp :type "PrimitiveComponent Object Reference") (OtherBodyIndex :type Integer) (bFromSweep :type Boolean) (SweepResult :type "HitResult Structure (by ref)"))
  (cast `/Game/FirstPerson/Blueprints/BP_FirstPersonCharacter` OtherActor)
  (`self.Show E Interact`)
  (`PrimitiveComponent.SetRenderCustomDepth` (`self.StaticMesh`) true))

(event `Show E Interact`
  ;[1 1 1] Interaction Pop Up && Visibility
  (if (not (`self.DontShowText`))
    (`SceneComponent.SetVisibility` (`self.Text Render`) true false)
    (`self.Text Facing Player`)))

(event `Text Facing Player`
  (bind _text_render (`self.Text Render`))
  ;[1 1 1] Interaction Pop Up && Visibility
  ;;[1 1 1] Text Facing Player
  (`KismetSystemLibrary.K2_SetTimerDelegate` (delegate `Text Facing Player`) 0.03 true)
  (`SceneComponent.K2_SetRelativeRotation` _text_render (`KismetMathLibrary.FindLookAtRotation` (`SceneComponent.K2_GetComponentLocation` _text_render) (`self.K2_GetActorLocation` (`GameplayStatics.GetPlayerPawn` 0))) false false))

(event `self.Box.OnComponentEndOverlap`
  (params (OverlappedComponent :type "PrimitiveComponent Object Reference") (OtherActor :type "Actor Object Reference") (OtherComp :type "PrimitiveComponent Object Reference") (OtherBodyIndex :type Integer))
  ;[1 1 1] Interaction Pop Up && Visibility
  (cast `/Game/FirstPerson/Blueprints/BP_FirstPersonCharacter` OtherActor)
  (`SceneComponent.SetVisibility` (`self.Text Render`) false false)
  (`PrimitiveComponent.SetRenderCustomDepth` (`self.StaticMesh`) false))

(event `/Game/Blueprints/BP_Object_Interactions_Interface.Object_Interaction`
  ;[1 1 1] Interaction Pop Up && Visibility
  (`SceneComponent.SetVisibility` (`self.Text Render`) false false)
  (bind _output_get (set `self.DontShowText` (not (`self.DontShowText`))))
  (if (not _output_get)
    (`self.Show E Interact`)))

(fn `UserConstructionScript`)